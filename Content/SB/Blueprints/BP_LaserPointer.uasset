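; BP_LaserPointer shows a Niagara laser beam for pointing at widgets through a widget interaction component.
; On BeginPlay it attaches NS_Pointer to LaserPos and starts a fast looping timer, apparently for length updates.
; UpdateParticleLength sets BeamEnd to the hit distance over hit-testable widgets, otherwise to the full interaction distance.
; DestroyPointer removes the spawned beam.
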(event Custom|SpawnPointerParticle
  (bind _returnvalue (Niagara|SpawnSystemAttached "/Game/SB/particle/NS_Pointer.NS_Pointer" (Variables|Default|GetlaserPos) "Pointer" "0, 0, 0" "0, 0, 0" "SnapToTarget" false))
  (Variables|Default|SetPointerSpawned _returnvalue))

(event Custom|DestroyPointer
  (bind _pointerspawned (Variables|Default|GetPointerSpawned))
  (Utilities|IsValid _pointerspawned
    (:Is%20Valid
      (Components|DestroyComponent _pointerspawned))))

(event Custom|UpdateParticleLength
  (bind _pointerspawned (Variables|Default|GetPointerSpawned))
  (bind _interactioncomp (Variables|Default|GetinteractionComp))
  (Utilities|IsValid _pointerspawned
    (:Is%20Valid
      (if (Class|WidgetInteractionComponent|IsOverHitTestVisibleWidget _interactioncomp)
        (Niagara|SetNiagaraVariable(Vector3) _pointerspawned "BeamEnd" (Math|Vector|MakeVector (.Distance (Collision|BreakHitResult (Class|WidgetInteractionComponent|GetLastHitResult _interactioncomp))) 0.0 0.0))
        (else
          (Niagara|SetNiagaraVariable(Vector3) _pointerspawned "BeamEnd" (Math|Vector|MakeVector (Variables|/Script/UMG.WidgetInteractionComponent|GetInteractionDistance _interactioncomp) 0.0 0.0)))))))

(event EventBeginPlay
  (CallFunction|SpawnPointerParticle)
  (Utilities|Time|SetTimerbyEvent (EventDispatchers|CreateEvent :!event Custom|UpdateParticleLength) 0.1 true))

(fn ConstructionScript)