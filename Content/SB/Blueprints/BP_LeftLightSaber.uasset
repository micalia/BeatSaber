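; Left lightsaber actor that stores Horizontal and Vertical input axis values for steering.
; An unconnected chain would combine them into a direction from the actor's right and inverted forward vectors, orient SmPointVal along it, and move the actor at Speed with sweep and clamped Y/Z bounds.
; Tick is empty and that chain never runs, so the saber does not move or rotate from this graph.
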(event EventBeginPlay)

(event Collision|EventActorBeginOverlap
  (params (OtherActor :type Actor%20Object%20Reference)))

(event EventTick
  (params (DeltaSeconds :type Float%20%28single-precision%29)))

(event Input|AxisEvents|InputAxisHorizontal
  (params (AxisValue :type Float%20%28single-precision%29))
  (Variables|Default|Seth AxisValue))

(event Input|AxisEvents|InputAxisVertical
  (params (AxisValue :type Float%20%28single-precision%29))
  (Variables|Default|Setv AxisValue))

(fn ConstructionScript)