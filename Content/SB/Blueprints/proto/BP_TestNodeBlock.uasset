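; BP_TestNodeBlock is a prototype test actor built around a static mesh and a procedural mesh.
; Its construction script copies the static mesh into the procedural mesh with collision.
; On BeginPlay it runs a Visibility line trace with persistent debug drawing and leaves the result unused.
; The trace ends at the scaled negative up vector without adding the actor location, so the endpoint is relative to the world origin.
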(event EventBeginPlay
  (Collision|LineTraceByChannel (Transformation|GetActorLocation) (* (* (Transformation|GetActorUpVector) (Class|KismetSystemLibrary|MakeLiteralInteger -1)) (Math|Float|MakeLiteralFloat 3e+02)) "TraceTypeQuery1" false 0 "Persistent"))

(event Collision|EventActorBeginOverlap
  (params (OtherActor :type Actor%20Object%20Reference)))

(event EventTick
  (params (DeltaSeconds :type Float%20%28single-precision%29)))

(fn ConstructionScript
  (Class|KismetProceduralMeshLibrary|CopyProceduralMeshfromStaticMeshComponent (Variables|Default|GetStaticMesh) 0 (Variables|Default|GetProceduralMesh) true))