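; Prototype game mode that tests spawning a node and moving it along a lane from start to end point.
; BeginPlay spaces the start points along Y, derives end points offset along X, and marks both with debug spheres.
; Tick spawns a node at the first start point after a delay, lerps it to its end over a set time, destroys it and repeats.
; Only the first lane is driven, one node at a time.
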(event EventBeginPlay
  (Utilities|FlowControl|Sequence
    (:then_0
      ;[1 1 1] 노드 시작 위치 만들기
      (for (_array_element _array_index) (Variables|Default|GetStartNodeLoc)
        (Utilities|Array|SetArrayElem (Variables|Default|GetStartNodeLoc) _array_index (Math|Vector|MakeVector (.X (Class|KismetMathLibrary|BreakVector3f _array_element)) (+ (.Y (Class|KismetMathLibrary|BreakVector3f _array_element)) (* (Variables|Default|GetLocGap) _array_index)) (Variables|Default|GetSpawnZaxis))))
      (for _array_element_2 (Variables|Default|GetStartNodeLoc)
        (Rendering|Debug|DrawDebugSphere _array_element_2 1e+02 12 "(R=0.000000,G=0.653586,B=1.000000,A=1.000000)" 2e+02)))
    (:then_1
      ;[1 1 1] 끝지점 노드 위치 만들기
      (for (_array_element_3 _array_index_2) (Variables|Default|GetStartNodeLoc)
        (Utilities|Array|SetArrayElem (Variables|Default|GetEndNodeLoc) _array_index_2 (Math|Vector|MakeVector (- (.X (Class|KismetMathLibrary|BreakVector3f _array_element_3)) (Variables|Default|GetDistance)) (.Y (Class|KismetMathLibrary|BreakVector3f _array_element_3)) (.Z (Class|KismetMathLibrary|BreakVector3f _array_element_3)))))
      (for _array_element_4 (Variables|Default|GetEndNodeLoc)
        (Rendering|Debug|DrawDebugSphere _array_element_4 1e+02 12 "(R=1.000000,G=0.000000,B=0.057804,A=1.000000)" 2e+02)))))

(event EventTick
  (params (DeltaSeconds :type Float%20%28single-precision%29))
  (Utilities|FlowControl|Sequence
    (:then_0
      (Utilities|IsValid (Variables|Default|GetNode1)
        (:Is%20Valid
          (Development|PrintString "IsValid"))
        (:Is%20Not%20Valid
          (Development|PrintString "IsNotValid")
          (bind _output_get (Variables|Default|SetSpawnCurrTime (+ DeltaSeconds (Variables|Default|GetSpawnCurrTime))))
          (if (> _output_get (Variables|Default|GetSpawnDelay))
            (Variables|Default|SetSpawnCurrTime 0.0)
            (bind _returnvalue (Game|SpawnActorfromClass (Variables|Default|GetSpawnNode) (Math|Transform|MakeTransform (Utilities|Array|Get(acopy) (Variables|Default|GetStartNodeLoc)) "0, 0, 0" "1.000000,1.000000,1.000000") "Undefined" "MultiplyWithRoot" 0 0))
            (Variables|Default|SetNode1 _returnvalue)))))
    (:then_1
      (Utilities|IsValid (Variables|Default|GetNode1)
        (:Is%20Valid
          (bind _output_get_2 (Variables|Default|SetMoveCurrTime (+ DeltaSeconds (Variables|Default|GetMoveCurrTime))))
          (bind _output_get_3 (Variables|Default|SetMoveAlpha (/ _output_get_2 (Variables|Default|GetMoveTime))))
          (if (> (Variables|Default|GetMoveAlpha) (Math|Float|MakeLiteralFloat 1.0))
            (Actor|DestroyActor (Variables|Default|GetNode1))
            (Variables|Default|SetMoveAlpha 0.0)
            (Variables|Default|SetMoveCurrTime 0.0)
            (else
              (Transformation|SetActorLocation (Variables|Default|GetNode1) (.Location (Math|Transform|BreakTransform (Math|Transform|Lerp(Transform) (Math|Transform|MakeTransform (Utilities|Array|Get(acopy) (Variables|Default|GetStartNodeLoc)) "0, 0, 0" "1.000000,1.000000,1.000000") (Math|Transform|MakeTransform (Utilities|Array|Get(acopy) (Variables|Default|GetEndNodeLoc)) "0, 0, 0" "1.000000,1.000000,1.000000") _output_get_3))) false false))))))))

(fn ConstructionScript)