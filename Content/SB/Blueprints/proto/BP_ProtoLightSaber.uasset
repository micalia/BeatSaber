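; Prototype lightsaber actor that moves with Horizontal and Vertical axis input and slices procedural meshes its blade passes through.
; Tick sweeps it along the input direction within clamped Y/Z bounds and turns the Point component to follow that direction.
; Blade begin overlap caches the procedural mesh through a DoOnce; end overlap cuts it on Point's plane, then applies physics and an impulse to the new capped half.
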(event OnComponentBeginOverlap(Blade)
  (params (OverlappedComponent :type Primitive%20Component%20Object%20Reference) (OtherActor :type Actor%20Object%20Reference) (OtherComp :type Primitive%20Component%20Object%20Reference) (OtherBodyIndex :type Integer) (bFromSweep :type Boolean) (SweepResult :type Hit%20Result%20Structure%20%28by%20ref%29))
  (Development|PrintString "Start")
  (Utilities|FlowControl|DoOnce false
    (:Completed
      (bind _asprocedural_mesh_component (Utilities|Casting|CastToProceduralMeshComponent OtherComp)))))

(event OnComponentEndOverlap(Blade)
  (params (OverlappedComponent :type Primitive%20Component%20Object%20Reference) (OtherActor :type Actor%20Object%20Reference) (OtherComp :type Primitive%20Component%20Object%20Reference) (OtherBodyIndex :type Integer))
  (bind _point (Variables|Default|GetPoint))
  (bind _returnvalue (Transformation|GetWorldLocation _point))
  (Development|PrintString "End")
  (Utilities|FlowControl|Sequence
    (:then_0
      (Utilities|FlowControl|DoOnce false) ; enters at Reset
    )
    (:then_1
      (Utilities|IsValid (stale OnComponentBeginOverlap(Blade) _asprocedural_mesh_component)
        (:Is%20Valid
          _)
        (:Is%20Not%20Valid
          _))
      (Rendering|Debug|DrawDebugSphere _returnvalue 2e+01 12 "(R=1.000000,G=0.000000,B=0.000000,A=1.000000)" 14.0 2.0)
      (bind _outotherhalfprocmesh (Class|KismetProceduralMeshLibrary|SliceProceduralMesh (stale OnComponentBeginOverlap(Blade) _asprocedural_mesh_component) _returnvalue (Math|Vector|GetUpVector _point) true "CreateNewSectionForCap" "/Game/SB/Models/light-saber/source/02_-_Default.02_-_Default"))
      (Physics|SetSimulatePhysics _outotherhalfprocmesh true)
      (Physics|AddImpulse _outotherhalfprocmesh "300.000000,300.000000,300.000000" "None" true))))

(event EventBeginPlay)

(event Collision|EventActorBeginOverlap
  (params (OtherActor :type Actor%20Object%20Reference)))

(event EventTick
  (params (DeltaSeconds :type Float%20%28single-precision%29))
  (bind _output_get (Variables|Default|Setdir (+ (* (Transformation|GetActorRightVector) (Variables|Default|Geth)) (* (* (Transformation|GetActorForwardVector) (Math|Float|MakeLiteralFloat -1.0)) (Variables|Default|Getv)))))
  (Transformation|SetWorldRotation (Variables|Default|GetPoint) (Class|KismetMathLibrary|MakeRotfromYX (Math|Vector|Normalize _output_get) (Math|Vector|GetUpVector (Variables|Default|GetScene))) false false)
  (Transformation|SetActorLocation (Math|Vector|MakeVector (.X (Class|KismetMathLibrary|BreakVector3f (+ (Transformation|GetActorLocation) (* (* (Math|Vector|Normalize _output_get) (Variables|Default|Getspeed)) DeltaSeconds)))) (Math|Float|Clamp(Float) (.Y (Class|KismetMathLibrary|BreakVector3f (+ (Transformation|GetActorLocation) (* (* (Math|Vector|Normalize _output_get) (Variables|Default|Getspeed)) DeltaSeconds)))) -4e+02 4e+02) (Math|Float|Clamp(Float) (.Z (Class|KismetMathLibrary|BreakVector3f (+ (Transformation|GetActorLocation) (* (* (Math|Vector|Normalize _output_get) (Variables|Default|Getspeed)) DeltaSeconds)))) 0.0 3.5e+02)) true false))

(event Input|AxisEvents|InputAxisHorizontal
  (params (AxisValue :type Float%20%28single-precision%29))
  (Variables|Default|Seth AxisValue))

(event Input|AxisEvents|InputAxisVertical
  (params (AxisValue :type Float%20%28single-precision%29))
  (Variables|Default|Setv AxisValue))

(fn ConstructionScript)