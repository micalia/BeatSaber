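; BP_InGameMode is a game mode Blueprint that runs the opening sequence before play starts.
; On BeginPlay it blends the view to the BP_VR_Player actor, possesses it and fades the camera in.
; After a delay matching the blend time, it sets the GameStart flag on InGameMode, calls GameStart and prints a start message.
; It also looks up BP_FirstCameraActor but does not use the result.
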(event EventBeginPlay
  (bind _delaytime (Variables|Default|GetdelayTime))
  (Actor|GetActorOfClass "/Game/SB/Blueprints/BP_FirstCameraActor.BP_FirstCameraActor_C")
  (bind _returnvalue (Actor|GetActorOfClass "/Game/SB/Blueprints/proto/BP_VR_Player.BP_VR_Player_C"))
  (Game|Player|SetViewTargetwithBlend (Game|GetPlayerController (Game|GetPlayerState 0)) _returnvalue _delaytime "VTBlend_EaseInOut" _delaytime false)
  (Pawn|Possess (Game|GetPlayerController 0) _returnvalue)
  (CameraFades|StartCameraFade :self (Game|GetPlayerCameraManager 0) :FromAlpha 1.0 :Duration 2.5)
  (Utilities|FlowControl|Delay (Variables|Default|GetdelayTime))
  (bind _asin_game_mode (Utilities|Casting|CastToInGameMode (Game|GetGameMode)))
  (Variables|/Script/BeatSaber.InGameMode|SetbGameStart _asin_game_mode true)
  (Class|InGameMode|GameStart)
  (Development|PrintString "Start!!!!!!"))

(fn ConstructionScript)