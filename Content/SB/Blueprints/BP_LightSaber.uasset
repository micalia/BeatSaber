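; BP_LightSaber is a player-steered lightsaber that moves at a set speed within a bounded area.
; Horizontal and Vertical input axes are stored and combined each Tick with the actor's right and negated forward vectors into a direction.
; That direction orients the SmPointVal component around the root's up vector and drives a swept move, with world Y and Z clamped to fixed limits.
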(event EventBeginPlay)

(event Collision|EventActorBeginOverlap
  (params (OtherActor :type Actor%20Object%20Reference)))

(event EventTick
  (params (DeltaSeconds :type Float%20%28single-precision%29))
  (bind _output_get (Variables|Default|Setdir (+ (* (Transformation|GetActorRightVector) (Variables|Default|Geth)) (* (* (Transformation|GetActorForwardVector) (Math|Float|MakeLiteralFloat -1.0)) (Variables|Default|Getv)))))
  (Transformation|SetWorldRotation (Variables|Default|Getsm_pointVal) (Class|KismetMathLibrary|MakeRotfromYX (Math|Vector|Normalize _output_get) (Math|Vector|GetUpVector (Variables|Default|GetrootComp))) false false)
  (Transformation|SetActorLocation (Math|Vector|MakeVector (.X (Class|KismetMathLibrary|BreakVector3f (+ (Transformation|GetActorLocation) (* (* (Math|Vector|Normalize _output_get) (Variables|Default|Getspeed)) DeltaSeconds)))) (Math|Float|Clamp(Float) (.Y (Class|KismetMathLibrary|BreakVector3f (+ (Transformation|GetActorLocation) (* (* (Math|Vector|Normalize _output_get) (Variables|Default|Getspeed)) DeltaSeconds)))) -4e+02 4e+02) (Math|Float|Clamp(Float) (.Z (Class|KismetMathLibrary|BreakVector3f (+ (Transformation|GetActorLocation) (* (* (Math|Vector|Normalize _output_get) (Variables|Default|Getspeed)) DeltaSeconds)))) -2.5e+02 2.5e+02)) true false))

(event Input|AxisEvents|InputAxisHorizontal
  (params (AxisValue :type Float%20%28single-precision%29))
  (Variables|Default|Seth AxisValue))

(event Input|AxisEvents|InputAxisVertical
  (params (AxisValue :type Float%20%28single-precision%29))
  (Variables|Default|Setv AxisValue))

(fn ConstructionScript)